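; AI_Butcher is an enemy pawn that wanders the level and chases the player once it spots them.
; While idle, Tick starts a move to a random navigable point nearby, using a Moving flag to wait until each move succeeds or fails.
; Pawn sensing sets an in-range flag that is never cleared, permanently stopping the wander, then moves toward the seen pawn if it is the player.
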(event OnSeePawn(PawnSensing)
  (params (Pawn :type Pawn%20Object%20Reference))
  (Variables|Default|Setinrange true)
  (bind _asplayer_main (Utilities|Casting|CastToPlayer_Main Pawn))
  (AI|AIMoveTo self "0, 0, 0" _asplayer_main 5.0 false))

(event EventTick
  (params (DeltaSeconds :type Float%20%28single-precision%29))
  (if (not (Variables|Default|Getinrange))
    (if (not (Variables|Default|Getmoving))
      (AI|AIMoveTo self (Class|NavigationSystem|GetRandomPointinNavigableRadius (Transformation|GetActorLocation) 1e+03) 0 5.0 false
        (:then
          (Variables|Default|Setmoving true))
        (:OnSuccess
          (Variables|Default|Setmoving false :!label _label))
        (:OnFail
          (goto _label))))))

(fn ConstructionScript)