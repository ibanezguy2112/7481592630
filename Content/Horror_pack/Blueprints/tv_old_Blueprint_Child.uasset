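; Child Blueprint of an old TV horror prop that switches on its lights and plays a TV sound.
; It starts on at BeginPlay when IsOn is set; otherwise it stays dark and silent until something overlaps its Trigger.
; The Trigger destroys itself on first overlap, making the scare one-shot.
; The spot and point lights turn off when the sound finishes playing.
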(event OnComponentBeginOverlap(trigger)
  (params (OverlappedComponent :type Primitive%20Component%20Object%20Reference) (OtherActor :type Actor%20Object%20Reference) (OtherComp :type Primitive%20Component%20Object%20Reference) (OtherBodyIndex :type Integer) (bFromSweep :type Boolean) (SweepResult :type Hit%20Result%20Structure%20%28by%20ref%29))
  (bind _tvcyclesound (Variables|Default|GetTvCycleSound))
  (Components|DestroyComponent (Variables|Default|Gettrigger))
  (if (not (Variables|Default|GetIs_on))
    (Rendering|SetVisibility (Variables|Default|GetSpotLight) true false)
    (Audio|Components|Audio|SetSound _tvcyclesound "/Game/Audio/Objects/TV/TvCycle.TvCycle")
    (Audio|Components|Audio|Play _tvcyclesound 0.0)))

(event OnAudioFinished(TvCycleSound)
  (Rendering|SetVisibility (Variables|Default|GetSpotLight) false false))

(event EventBeginPlay
  (bind _spotlight (Variables|Default|GetSpotLight))
  (bind _tvcyclesound (Variables|Default|GetTvCycleSound))
  (if (Variables|Default|GetIs_on)
    (Rendering|SetVisibility _spotlight true false)
    (Audio|Components|Audio|SetSound _tvcyclesound "/Game/Audio/Objects/TV/TvCycle.TvCycle")
    (Audio|Components|Audio|Play _tvcyclesound 0.0)
    (else
      (Rendering|SetVisibility _spotlight false false)
      (Audio|Components|Audio|Stop (Variables|Default|GetTvCycleSound)))))

(event Collision|EventActorBeginOverlap
  (params (OtherActor :type Actor%20Object%20Reference)))

(event EventTick
  (params (DeltaSeconds :type Float%20%28single-precision%29)))

(fn ConstructionScript
  (|CallParentFunction))